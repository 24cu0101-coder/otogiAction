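; Level-placed actor that plays the player's spawn-in effect when play begins in the Momotaro stage.
; On BeginPlay it hides player 0's character, disables its input and spawns the Player_Spawn particle system at the character's location.
; After a short delay it reveals the character and restores input.
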(event EventBeginPlay
  (bind _returnvalue (Game|GetPlayerCharacter 0))
  (bind _returnvalue_2 (Game|GetPlayerCharacter 0))
  (Rendering|SetActorHiddenInGame _returnvalue true)
  (Input|DisableInput _returnvalue (Game|GetPlayerController 0))
  (Niagara|SpawnSystematLocation "/Game/Effect/Spawn/Player_Spawn.Player_Spawn" (Transformation|GetActorLocation _returnvalue) "0.000000,-20.000000,0.000000")
  (Utilities|FlowControl|Delay 1.5)
  (Rendering|SetActorHiddenInGame _returnvalue_2 false)
  (Input|EnableInput _returnvalue_2 (Game|GetPlayerController 0)))

(fn ConstructionScript)