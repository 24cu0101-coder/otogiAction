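; Interactable level-select object in the Kanrikyoku game level.
; Overlapping Box1 toggles a widget component's visibility, while BP_NewPlayerCharacter1 entering Box enables this actor's input; leaving Box does not disable it.
; Left click or gamepad right face button then disables that input, hides the player, blends the view to this actor and opens WBP_LevelSelectUI in game-only input mode.
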(event OnComponentBeginOverlap(Box)
  (params (OverlappedComponent :type Primitive%20Component%20Object%20Reference) (OtherActor :type Actor%20Object%20Reference) (OtherComp :type Primitive%20Component%20Object%20Reference) (OtherBodyIndex :type Integer) (bFromSweep :type Boolean) (SweepResult :type Hit%20Result%20Structure%20%28by%20ref%29))
  (Utilities|Casting|CastToBP_NewPlayerCharacter1 OtherActor)
  (Variables|Default|SetPlayerRange "")
  (Input|EnableInput (Game|GetPlayerController 0)))

(event OnComponentBeginOverlap(Box1)
  (params (OverlappedComponent :type Primitive%20Component%20Object%20Reference) (OtherActor :type Actor%20Object%20Reference) (OtherComp :type Primitive%20Component%20Object%20Reference) (OtherBodyIndex :type Integer) (bFromSweep :type Boolean) (SweepResult :type Hit%20Result%20Structure%20%28by%20ref%29))
  (Rendering|SetVisibility (Variables|Default|GetWidget) true false))

(event OnComponentEndOverlap(Box1)
  (params (OverlappedComponent :type Primitive%20Component%20Object%20Reference) (OtherActor :type Actor%20Object%20Reference) (OtherComp :type Primitive%20Component%20Object%20Reference) (OtherBodyIndex :type Integer))
  (Rendering|SetVisibility (Variables|Default|GetWidget) false false))

(event Input|MouseEvents|LeftMouseButton
  (params (Key :type Key%20Structure :default "None"))
  (:Pressed
    (Input|DisableInput (Game|GetPlayerController 0))
    (Rendering|SetActorHiddenInGame (Game|GetPlayerCharacter 0) true)
    (Game|Player|SetViewTargetwithBlend (Game|GetPlayerController 0) self 0.0 "VTBlend_Linear" 0.0 false)
    (bind _returnvalue (UserInterface|CreateWidget "/Game/Level/GameLevel/Kanrikyoku/Widget/WBP_LevelSelectUI.WBP_LevelSelectUI_C"))
    (UserInterface|Viewport|AddtoViewport _returnvalue 0)
    (Input|SetInputModeGameOnly (Game|GetPlayerController 0) false)))

(event Input|GamepadEvents|GamepadFaceButtonRight
  (params (Key :type Key%20Structure :default "None"))
  (:Pressed
    (Input|DisableInput (Game|GetPlayerController 0))
    (Rendering|SetActorHiddenInGame (Game|GetPlayerCharacter 0) true)
    (Game|Player|SetViewTargetwithBlend (Game|GetPlayerController 0) self 0.0 "VTBlend_Linear" 0.0 false)
    (bind _returnvalue (UserInterface|CreateWidget "/Game/Level/GameLevel/Kanrikyoku/Widget/WBP_LevelSelectUI.WBP_LevelSelectUI_C"))
    (UserInterface|Viewport|AddtoViewport _returnvalue 0)
    (Input|SetInputModeGameOnly (Game|GetPlayerController 0) false)))

(fn ConstructionScript)